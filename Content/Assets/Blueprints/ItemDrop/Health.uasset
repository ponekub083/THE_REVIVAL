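; Health pickup Blueprint that heals the player character on collision and expires on its own.
; On Hit, it casts the other actor to Ue4ASP_Character_Ratation_Joys and adds HealPoint to its HPP, capped at MAXHP.
; It then spawns the Bullet particle emitter at its location and destroys itself.
; A Delay of SDestroy, driven from Tick rather than BeginPlay, destroys uncollected pickups.
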(event `self.ReceiveTick`
  (params (DeltaSeconds :type "Float (single-precision)"))
  (`KismetSystemLibrary.Delay` (`self.S_Destroy`))
  (`self.K2_DestroyActor`))

(event `self.ReceiveHit`
  (params (MyComp :type "PrimitiveComponent Object Reference") (Other :type "Actor Object Reference") (OtherComp :type "PrimitiveComponent Object Reference") (bSelfMoved :type Boolean) (HitLocation :type "Vector Structure") (HitNormal :type "Vector Structure") (NormalImpulse :type "Vector Structure") (Hit :type "HitResult Structure (by ref)"))
  (bind _asue_4asp_character_ratation_joys (cast `/Game/Assets/Blueprints/Character/Player/Ue4ASP_Character_Ratation_Joys` Other))
  (bind _returnvalue (+ (`/Game/Assets/Blueprints/Character/Player/Ue4ASP_Character_Ratation_Joys.HP_P` _asue_4asp_character_ratation_joys) (`KismetMathLibrary.Conv_IntToDouble` (`self.Heal Point`))))
  (bind _maxhp (`/Game/Assets/Blueprints/Character/Player/Ue4ASP_Character_Ratation_Joys.MAXHP` _asue_4asp_character_ratation_joys))
  (if (> _returnvalue _maxhp)
    (set `/Game/Assets/Blueprints/Character/Player/Ue4ASP_Character_Ratation_Joys.HP_P` _maxhp _asue_4asp_character_ratation_joys)
    (else
      (set `/Game/Assets/Blueprints/Character/Player/Ue4ASP_Character_Ratation_Joys.HP_P` _returnvalue _asue_4asp_character_ratation_joys)))
  (`GameplayStatics.SpawnEmitterAtLocation` "/Game/Assets/Blueprints/Weapon/Bullet/Material/bullet.bullet" (`self.K2_GetActorLocation` self))
  (`self.K2_DestroyActor`))

(fn `UserConstructionScript`)